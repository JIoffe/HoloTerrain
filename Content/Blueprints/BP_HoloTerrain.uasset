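; Holographic terrain actor that players sculpt with tagged hand meshes, using UXT input simulation meshes in editor.
; Construction builds a welded procedural grid whose material reads a persistent R32f heightmap.
; Each tick, an orthographic scene capture renders only those meshes with a temporarily swapped displacer material that samples the persistent heightmap, then copies the result back, forming a ping-pong buffer.
; Functions also provide smoothing, randomization, light rotation and toggleable grab manipulation.
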(event EventBeginPlay
  (bind _scenecapturecomponent2d (Variables|Default|GetSceneCaptureComponent2D))
  (bind _terrainresolution (Variables|Default|GetTerrainResolution))
  (Utilities|FlowControl|Sequence
    (:then_0
      ;[1 1 1] Create render targets for swap chain
      (bind _returnvalue (Rendering|CreateRenderTarget2D _terrainresolution _terrainresolution "RTF_R32f"))
      (bind _output_get (Variables|Default|SetRenderTarget _returnvalue))
      (Variables|/Script/Engine.Texture|SetSRGB _output_get false)
      (Rendering|ClearRenderTarget2D _output_get "(R=1.000000,G=1.000000,B=1.000000,A=1.000000)")
      (Variables|/Script/Engine.SceneCaptureComponent2D|SetTextureTarget (Variables|Default|GetSceneCaptureComponent2D) _output_get)
      (bind _returnvalue_2 (Rendering|CreateRenderTarget2D _terrainresolution _terrainresolution "RTF_R32f"))
      (bind _output_get_2 (Variables|Default|SetRenderTargetPersist _returnvalue_2))
      (Variables|/Script/Engine.Texture|SetSRGB _output_get_2 false)
      (Rendering|ClearRenderTarget2D _output_get_2 "(R=1.000000,G=1.000000,B=1.000000,A=1.000000)")
      (Rendering|Material|SetTextureParameterValue (Variables|Default|GetTerrainMaterial) "Heightmap" _output_get_2)
      (CallFunction|SetTerrainBrush))
    (:then_1
      (CallFunction|SeekSculptMeshes)
      (for _array_element (Variables|Default|GetSculptMeshes)
        (Rendering|SceneCapture|ShowOnlyComponent _scenecapturecomponent2d _array_element)
        (Variables|/Script/Engine.SceneCaptureComponent2D|SetOrthoWidth _scenecapturecomponent2d (Variables|Default|GetTerrainWidth))))
    (:then_2
      ;[1 1 1] Material instances for sculpting meshes and frame buffer
      (bind _returnvalue_3 (Rendering|Material|CreateDynamicMaterialInstance "/Game/Materials/M_TerrainDisplacer.M_TerrainDisplacer" "None" "None" :!class /Script/Engine.KismetMaterialLibrary))
      (bind _output_get_3 (Variables|Default|SetSculptMaterialDynamic _returnvalue_3))
      (Rendering|Material|SetTextureParameterValue _output_get_3 "HeightMap" (Variables|Default|GetRenderTargetPersist))
      (bind _returnvalue_4 (Rendering|Material|CreateDynamicMaterialInstance "/Game/Materials/M_Blur.M_Blur" "None" "None" :!class /Script/Engine.KismetMaterialLibrary))
      (bind _output_get_4 (Variables|Default|SetBlurMaterial _returnvalue_4))
      (Rendering|Material|SetTextureParameterValue _output_get_4 "Texture" (Variables|Default|GetRenderTargetPersist))
      (bind _returnvalue_5 (Rendering|Material|CreateDynamicMaterialInstance "/Game/Materials/M_RandomIsland.M_RandomIsland" "None" "None" :!class /Script/Engine.KismetMaterialLibrary))
      (Variables|Default|SetRandomTerrainMaterial _returnvalue_5))))

(event EventTick
  (params (DeltaSeconds :type Float%20%28single-precision%29))
  (Transformation|SetActorRotation (Math|Rotator|MakeRotator 0.0 0.0 (.Yaw (Math|Rotator|BreakRotator (Transformation|GetActorRotation)))))
  (CallFunction|UpdateHeightmap))

(fn ConstructionScript
  (CallFunction|GenerateTerrainMesh))

(fn UpdateHeightmap
  (CallFunction|SetCaptureMaterials)
  (Rendering|SceneCapture|CaptureScene (Variables|Default|GetSceneCaptureComponent2D) :!class /Script/Engine.SceneCaptureComponent2D)
  (CallFunction|ResetMaterials)
  (CallFunction|CopytoPersistentBuffer))

(fn SeekSculptMeshes
  (bind _returnvalue (Game|Player|GetPlayerPawn 0))
  (Utilities|FlowControl|Sequence
    (:then_0
      (if (Class|UxtFunctionLibrary|IsinEditor)
        ;[1 1 1] Get Simulation Actor Meshes (if running in editor)
        (bind _outactors (Actor|GetAllActorsOfClass "/Script/UXToolsInputSimulation.UxtInputSimulationActor"))
        (for _array_element _outactors
          (Utilities|FlowControl|Sequence
            (:then_0
              (for _array_element_2 (Actor|GetComponentsbyTag _array_element "/Script/Engine.ActorComponent" "Left")
                (bind _asmesh_component (Utilities|Casting|CastToMeshComponent _array_element_2))
                (Utilities|Array|Add (Variables|Default|GetSculptMeshes) _asmesh_component)))
            (:then_1
              (for _array_element_3 (Actor|GetComponentsbyTag _array_element "/Script/Engine.ActorComponent" "Right")
                (bind _asmesh_component_2 (Utilities|Casting|CastToMeshComponent _array_element_3))
                (Utilities|Array|Add (Variables|Default|GetSculptMeshes) _asmesh_component_2)))))
        (else
          ;[1 1 1] Get hand meshes from pawn
          (Utilities|FlowControl|Sequence
            (:then_0
              (for _array_element_4 (Actor|GetComponentsbyTag _returnvalue "/Script/Engine.ActorComponent" "Left")
                (bind _asmesh_component_3 (Utilities|Casting|CastToMeshComponent _array_element_4))
                (Utilities|Array|Add (Variables|Default|GetSculptMeshes) _asmesh_component_3)))
            (:then_1
              (for _array_element_5 (Actor|GetComponentsbyTag _returnvalue "/Script/Engine.ActorComponent" "Right")
                (bind _asmesh_component_4 (Utilities|Casting|CastToMeshComponent _array_element_5))
                (Utilities|Array|Add (Variables|Default|GetSculptMeshes) _asmesh_component_4)))))))
    (:then_1
      ;[1 1 1] Cache original materials to switch back after displacement capture
      (for _array_element_6 (Variables|Default|GetSculptMeshes)
        (Utilities|Array|Add (Variables|Default|GetSculptMeshMaterials) (Rendering|Material|GetMaterial _array_element_6 0))))))

(fn SetCaptureMaterials
  (bind _sculptmaterialdynamic (Variables|Default|GetSculptMaterialDynamic))
  (Utilities|FlowControl|Sequence
    (:then_0
      (Rendering|Material|SetScalarParameterValue _sculptmaterialdynamic "MaxHeight" (Variables|Default|GetMaxHeight) :!class /Script/Engine.MaterialInstanceDynamic)
      (bind _extents (CallFunction|GetXYExtents))
      (Rendering|Material|SetVectorParameterValue _sculptmaterialdynamic "Extents" _extents :!class /Script/Engine.MaterialInstanceDynamic))
    (:then_1
      (for _array_element (Variables|Default|GetSculptMeshes)
        (Rendering|Material|SetMaterial _array_element 0 (Variables|Default|GetSculptMaterialDynamic))))))

(fn ResetMaterials
  (for (_array_element _array_index) (Variables|Default|GetSculptMeshes)
    (Rendering|Material|SetMaterial _array_element 0 (Utilities|Array|Get(acopy) (Variables|Default|GetSculptMeshMaterials) _array_index))))

(fn GetXYExtents
  (bind _returnvalue (Transformation|GetActorLocation))
  (bind _terrainwidth (Variables|Default|GetTerrainWidth))
  (bind _returnvalue_2 (* _terrainwidth 0.5))
  (return (Utilities|Struct|MakeLinearColor (- (.x _returnvalue) _returnvalue_2) (- (.y _returnvalue) _returnvalue_2) (.z _returnvalue) (/ 1.0 _terrainwidth))))

(fn GenerateTerrainMesh
  (bind _terrain (Variables|Default|GetTerrain))
  (bind _terrainresolution (Variables|Default|GetTerrainResolution))
  (bind (_triangles _vertices _uvs) (Class|KismetProceduralMeshLibrary|CreateGridMeshWelded _terrainresolution _terrainresolution (/ (Variables|Default|GetTerrainWidth) (Math|Conversions|ToFloat(Integer) _terrainresolution))))
  (Class|ProceduralMeshComponent|CreateMeshSectionLinearColor _terrain 0 _vertices _triangles 0 _uvs 0 0 0 0 0 false)
  (bind _returnvalue (Rendering|Material|CreateDynamicMaterialInstance "/Game/Materials/M_Terrain.M_Terrain" "None" "None" :!class /Script/Engine.KismetMaterialLibrary))
  (bind _output_get (Variables|Default|SetTerrainMaterial _returnvalue))
  (Rendering|Material|SetScalarParameterValue _output_get "MaxHeight" (Variables|Default|GetMaxHeight) :!class /Script/Engine.MaterialInstanceDynamic)
  (Rendering|Material|SetScalarParameterValue _output_get "Texel" (/ 1.0 (Math|Conversions|ToFloat(Integer) (Variables|Default|GetTerrainResolution))) :!class /Script/Engine.MaterialInstanceDynamic)
  (Rendering|Material|SetScalarParameterValue _output_get "VStep" 15.0 :!class /Script/Engine.MaterialInstanceDynamic)
  (Rendering|Material|SetMaterial _terrain 0 _output_get))

(fn SetTerrainBrush
  (params (BrushMaterial :type Material%20Instance%20Object%20Reference))
  (Utilities|IsValid BrushMaterial
    (:Is%20Valid
      (Rendering|DrawMaterialtoRenderTarget (Variables|Default|GetRenderTarget) BrushMaterial)
      (Rendering|DrawMaterialtoRenderTarget (Variables|Default|GetRenderTargetPersist) BrushMaterial))
    (:Is%20Not%20Valid
      (Rendering|DrawMaterialtoRenderTarget (Variables|Default|GetRenderTarget) "/Game/Materials/M_TerrainBrush.M_TerrainBrush")
      (Rendering|DrawMaterialtoRenderTarget (Variables|Default|GetRenderTargetPersist) "/Game/Materials/M_TerrainBrush.M_TerrainBrush"))))

(fn RotateLight
  (params (DeltaSeconds :type Float%20%28single-precision%29))
  (bind _output_get (Variables|Default|SetLightVectorWorld (Math|Vector|RotateVectorAroundAxis (Variables|Default|GetLightVectorWorld) (* DeltaSeconds (Variables|Default|GetLightRotateSpeed)) (Math|Vector|VectorUp))))
  (Rendering|Material|SetVectorParameterValue (Variables|Default|GetTerrainMaterial) "LightWorld" (Math|Conversions|ToLinearColor(Vector) _output_get) :!class /Script/Engine.MaterialInstanceDynamic))

(fn ToggleMoveTerrain
  (params (AllowMoveTerrain :type Boolean))
  (bind _uxtgenericmanipulator (Variables|Default|GetUxtGenericManipulator))
  (if AllowMoveTerrain
    (Variables|/Script/UXTools.UxtGrabTargetComponent|SetInteractionMode _uxtgenericmanipulator 3)
    (Variables|/Script/UXTools.UxtGrabTargetComponent|SetGrabModes _uxtgenericmanipulator 3)
    (else
      (Variables|/Script/UXTools.UxtGrabTargetComponent|SetInteractionMode _uxtgenericmanipulator 0)
      (Variables|/Script/UXTools.UxtGrabTargetComponent|SetGrabModes _uxtgenericmanipulator 0))))

(fn SmoothTerrain
  (Rendering|DrawMaterialtoRenderTarget (Variables|Default|GetRenderTarget) (Variables|Default|GetBlurMaterial))
  (CallFunction|CopytoPersistentBuffer))

(fn RandomizeTerrain
  (bind _randomterrainmaterial (Variables|Default|GetRandomTerrainMaterial))
  (Rendering|Material|SetScalarParameterValue _randomterrainmaterial "Seed" (Actor|GetGameTimeSinceCreation) :!class /Script/Engine.MaterialInstanceDynamic)
  (CallFunction|SetTerrainBrush _randomterrainmaterial))

(fn CopytoPersistentBuffer
  (bind (_canvas _size _context) (Rendering|BeginDrawCanvastoRenderTarget (Variables|Default|GetRenderTargetPersist)))
  (Canvas|DrawTexture :self _canvas :RenderTexture (Variables|Default|GetRenderTarget) :ScreenSize _size :CoordinateSize "(X=1.000000,Y=1.000000)" :BlendMode "BLEND_Opaque" :PivotPoint "(X=0.500000,Y=0.500000)")
  (Rendering|EndDrawCanvastoRenderTarget _context))