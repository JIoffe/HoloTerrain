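; BP_PalmMenu is a mixed reality hand menu built on UX Tools that appears on a palm-up gesture and adjusts the scene's water level.
; The palm-up constraint shows or hides the UI element and notifies the MRPawn of each menu toggle.
; The water level slider forwards its value to the BP_WaterPlane actor found at BeginPlay.
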(event OnConstraintActivated(UxtPalmUpConstraint)
  (Class|UxtUIElementComponent|SetUIVisibility (Variables|Default|GetUxtUIElement) "Show")
  (bind _asmrpawn (Utilities|Casting|CastToMRPawn (Game|Player|GetPlayerPawn 0)))
  (Default|OnMenuToggleEvent _asmrpawn true))

(event OnConstraintDeactivated(UxtPalmUpConstraint)
  (Class|UxtUIElementComponent|SetUIVisibility (Variables|Default|GetUxtUIElement) "Hide")
  (bind _asmrpawn (Utilities|Casting|CastToMRPawn (Game|Player|GetPlayerPawn 0)))
  (Default|OnMenuToggleEvent _asmrpawn false))

(event OnUpdateValue(WaterLevelSlider)
  (params (Slider :type Uxt%20Pinch%20Slider%20Component%20Object%20Reference) (NewValue :type Float%20%28single-precision%29))
  (Default|WaterLevelAdjustedEvent (Variables|Default|GetWaterPlane) NewValue))

(event EventBeginPlay
  (bind _returnvalue (Actor|GetActorOfClass "/Game/Blueprints/BP_WaterPlane.BP_WaterPlane_C"))
  (Variables|Default|SetWaterPlane _returnvalue))

(fn ConstructionScript)