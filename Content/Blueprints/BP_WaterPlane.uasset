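; BP_WaterPlane is the water surface for BP_HoloTerrain, spawning ripples where tracked hands dip below it.
; On BeginPlay it pre-spawns one silent Niagara ripple system per hand keypoint.
; Tick moves submerged keypoints' emitters to the surface and toggles spawn rate by height alone, without checking plane bounds.
; A water-level event sets the actor's height from the terrain's base and MaxHeight.
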(event Custom|WaterLevelAdjusted_Event
  (params (WaterLevel :type Float%20%28single-precision%29))
  (CallFunction|UpdateWaterLevel WaterLevel))

(event EventBeginPlay
  (Utilities|FlowControl|Sequence
    (:then_0
      (for _array_element (Variables|Default|GetTargetHands)
        (for _array_element_2 (Variables|Default|GetTargetHandKeypoints)
          (bind _returnvalue (Niagara|SpawnSystematLocation "/Game/FX/FX_WaterRipples.FX_WaterRipples" (+ (Transformation|GetWorldLocation (Variables|Default|GetPlane)) "0, 0,0.010000")))
          (Niagara|SetNiagaraVariable(Float) _returnvalue "User.SpawnRate" 0.0)
          (Utilities|Array|Add (Variables|Default|GetRippleEmitters) _returnvalue))))
    (:then_1
      (bind _returnvalue_2 (Actor|GetActorOfClass "/Game/Blueprints/BP_HoloTerrain.BP_HoloTerrain_C"))
      (Variables|Default|SetTerrain _returnvalue_2))
    (:then_2
      (EventDispatchers|BindEventtoWaterLevelAdjusted (delegate Custom|WaterLevelAdjusted_Event)))))

(event EventTick
  (params (DeltaSeconds :type Float%20%28single-precision%29))
  (bind _targethandkeypoints (Variables|Default|GetTargetHandKeypoints))
  (bind _plane (Variables|Default|GetPlane))
  (bind _returnvalue (Transformation|GetWorldLocation _plane))
  (for (_array_element _array_index) (Variables|Default|GetTargetHands)
    (bind _motioncontrollerdata (Class|HeadMountedDisplayFunctionLibrary|GetMotionControllerData 0 _array_element))
    (if (and (.bValid (Utilities|Struct|BreakXRMotionControllerData _motioncontrollerdata)) (Utilities|Enum|Equal(Enum) (.DeviceVisualType (Utilities|Struct|BreakXRMotionControllerData _motioncontrollerdata)) "Hand"))
      (for (_array_element_2 _array_index_2) _targethandkeypoints
        (if (< (.z (Utilities|Array|Get(acopy) (.HandKeyPositions (Utilities|Struct|BreakXRMotionControllerData _motioncontrollerdata)) (Math|Conversions|ToInteger(Byte) _array_element_2))) (.z _returnvalue))
          (Transformation|SetWorldLocation (Utilities|Array|Get(acopy) (Variables|Default|GetRippleEmitters) (+ (* _array_index (Utilities|Array|Length _targethandkeypoints)) _array_index_2)) (Math|Vector|MakeVector (.x (Utilities|Array|Get(acopy) (.HandKeyPositions (Utilities|Struct|BreakXRMotionControllerData _motioncontrollerdata)) (Math|Conversions|ToInteger(Byte) _array_element_2))) (.y (Utilities|Array|Get(acopy) (.HandKeyPositions (Utilities|Struct|BreakXRMotionControllerData _motioncontrollerdata)) (Math|Conversions|ToInteger(Byte) _array_element_2))) (+ (.z _returnvalue) 0.01)) false false)
          (Effects|Components|ParticleSystem|SetFloatParameter (Utilities|Array|Get(acopy) (Variables|Default|GetRippleEmitters) (+ (* _array_index (Utilities|Array|Length _targethandkeypoints)) _array_index_2)) "User.SpawnRate" 4.0)
          (else
            (Effects|Components|ParticleSystem|SetFloatParameter (Utilities|Array|Get(acopy) (Variables|Default|GetRippleEmitters) (+ (* _array_index (Utilities|Array|Length _targethandkeypoints)) _array_index_2)) "User.SpawnRate" 0.0)))))))

(fn ConstructionScript)

(fn UpdateWaterLevel
  (params (WaterLevel :type Float%20%28single-precision%29))
  (bind _returnvalue (Transformation|GetActorLocation))
  (bind _terrain (Variables|Default|GetTerrain))
  (Transformation|SetActorLocation (Math|Vector|MakeVector (.x _returnvalue) (.y _returnvalue) (+ (* WaterLevel (Variables|/Game/Blueprints/BP_HoloTerrain.BP_HoloTerrain_C|GetMaxHeight _terrain)) (.z (Transformation|GetWorldLocation (Variables|/Game/Blueprints/BP_HoloTerrain.BP_HoloTerrain_C|GetTerrain _terrain))))) false false))