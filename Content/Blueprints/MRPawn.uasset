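; Mixed reality player pawn that shows tracked hands and spawns a UXT hand interaction actor for each hand, plus a palm menu.
; Each tick it copies tracked joint poses onto two posable hand meshes, using bone names built from the joint enum and a negative Y scale for the left hand.
; Hands hide when tracking is lost, and opening the palm menu hides both meshes and pauses their updates.
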(event Custom|OnMenuToggle_Event
  (params (IsVisible :type Boolean))
  (Variables|Default|SetShouldUpdateHandMeshes (not IsVisible))
  (Development|SetHiddeninGame (Variables|Default|GetRightHand) IsVisible false)
  (Development|SetHiddeninGame (Variables|Default|GetLeftHand) IsVisible false))

(event EventBeginPlay
  (bind _returnvalue (Math|Transform|MakeTransform "0, 0, 0"))
  (bind _self self)
  (Utilities|FlowControl|Sequence
    (:then_0
      (for _array_element (Variables|Default|GetHandJoints)
        (Utilities|Array|Add (Variables|Default|GetHandJointNames) (Utilities|String|StringToName (Utilities|String|Replace (Utilities|String|EnumtoString _array_element) " ")))))
    (:then_1
      (Game|SpawnActorfromClass "/Game/Blueprints/BP_PalmMenu.BP_PalmMenu_C" (Math|Transform|MakeTransform "0, 0, 0") "Undefined" self 0)
      (EventDispatchers|BindEventtoOnMenuToggle (delegate Custom|OnMenuToggle_Event)))
    (:then_2
      (bind _returnvalue_2 (Game|SpawnActorfromClass "/Script/UXTools.UxtHandInteractionActor" _returnvalue "Undefined" _self false "Left" 0))
      (bind _output_get (Variables|Default|SetLeftHandInteraction _returnvalue_2))
      (Rendering|SetActorHiddenInGame _output_get true)
      (bind _returnvalue_3 (Game|SpawnActorfromClass "/Script/UXTools.UxtHandInteractionActor" _returnvalue "Undefined" _self false "Right" 0))
      (bind _output_get_2 (Variables|Default|SetRightHandInteraction _returnvalue_3))
      (Rendering|SetActorHiddenInGame _output_get_2 false))))

(event EventTick
  (params (DeltaSeconds :type Float%20%28single-precision%29))
  (if (Variables|Default|GetShouldUpdateHandMeshes)
    (CallFunction|UpdateRightHand)
    (CallFunction|UpdateLeftHand)))

(fn ConstructionScript)

(fn UpdateRightHand
  (bind _righthand (Variables|Default|GetRightHand))
  (for (_array_element _array_index) (Variables|Default|GetHandJoints)
    (bind (_outorientation _outposition _outradius _returnvalue) (Class|UxtHandTrackingFunctionLibrary|GetHandJointState "Right" _array_element))
    (Development|SetHiddeninGame _righthand (not _returnvalue) false)
    (if _returnvalue
      (Components|PoseableMesh|SetBoneTransformbyName _righthand (Utilities|Array|Get(acopy) (Variables|Default|GetHandJointNames) _array_index) (Math|Transform|ComposeTransforms (Math|Transform|MakeTransform _outposition (Class|KismetMathLibrary|QuatRotator _outorientation)) (Transformation|GetWorldTransform _righthand)) "ComponentSpace"))))

(fn UpdateLeftHand
  (bind _lefthand (Variables|Default|GetLeftHand))
  (for (_array_element _array_index) (Variables|Default|GetHandJoints)
    (bind (_outorientation _outposition _outradius _returnvalue) (Class|UxtHandTrackingFunctionLibrary|GetHandJointState "Left" _array_element))
    (Development|SetHiddeninGame _lefthand (not _returnvalue) false)
    (if _returnvalue
      (Components|PoseableMesh|SetBoneTransformbyName _lefthand (Utilities|Array|Get(acopy) (Variables|Default|GetHandJointNames) _array_index) (Math|Transform|ComposeTransforms (Math|Transform|MakeTransform _outposition (Class|KismetMathLibrary|QuatRotator _outorientation) "1,-1.000000,1") (Transformation|GetWorldTransform _lefthand)) "ComponentSpace"))))

(fn EnableHandActor
  (params (InteractionActor :type Uxt%20Hand%20Interaction%20Actor%20Object%20Reference) (Active :type Boolean))
  (Rendering|SetActorHiddenInGame InteractionActor (not Active))
  (Actor|Tick|SetActorTickEnabled InteractionActor Active))